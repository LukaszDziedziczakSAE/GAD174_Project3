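; Modular character Blueprint that builds its body from a DT_Characters row, selected on BeginPlay with a fixed default.
; UpdateMesh applies either one full mesh or separate head and body-part meshes, plus the row's AnimBP.
; Body and equipment components follow the main Mesh via leader pose.
; Slot visibility toggles material sections by slot-name substring in full-mesh mode, or tagged components otherwise.
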(event EventBeginPlay
  (CallFunction|SetCharacter "NewEnumerator9"))

(fn ConstructionScript
  (Components|SkinnedMesh|SetLeaderPoseComponent (Variables|Default|GetBody_Feet) (Variables|Character|GetMesh) true false))

(fn SetCharacter
  (params (Character :type ECharacter%20Enum :default "NewEnumerator0"))
  (Variables|Default|SetCharacter Character)
  (Utilities|FlowControl|Sequence
    (:then_0
      (bind _outrownames (DataTable|GetDataTableRowNames "/Game/ROG_Modular_Armor/Characters/Blueprints/DT_Characters.DT_Characters"))
      (for _array_element _outrownames
        (bind _returnvalue (Utilities|GetDataTableRow "/Game/ROG_Modular_Armor/Characters/Blueprints/DT_Characters.DT_Characters" _array_element)
          (:then
            (if (Utilities|Enum|Equal(Enum) (Utilities|Struct|BreakSCharacter _returnvalue) (Variables|Default|GetCharacter))
              (Variables|Default|SetCharacterInfo _returnvalue))))))
    (:then_1
      (CallFunction|UpdateMesh))))

(fn UpdateMesh
  (if (CallFunction|IsUseMaterialSlots)
    (CallFunction|SetFullMesh)
    (else
      (CallFunction|SetPartMesh))))

(fn IsUseMaterialSlots
  (return (Variables|Default|GetUseMaterialSlot)))

(fn SetFullMesh
  (bind _characterinfo (Variables|Default|GetCharacterInfo))
  (bind (_fullmesh _animbp) (Utilities|Struct|BreakSCharacter _characterinfo))
  (Components|SkinnedMesh|SetSkinnedAssetandUpdate (Variables|Character|GetMesh) _fullmesh true)
  (Components|SkinnedMesh|SetSkinnedAssetandUpdate (Variables|Default|GetBody_Feet) 0 true)
  (Class|SkeletalMeshComponent|SetAnimClass (Variables|Character|GetMesh) _animbp))

(fn SetPartMesh
  (bind _characterinfo (Variables|Default|GetCharacterInfo))
  (bind (_character _headmesh _chestmesh _armsmesh _handsmesh _feetmesh _legsmesh _animbp) (Utilities|Struct|BreakSCharacter _characterinfo))
  (if (Utilities|Enum|Equal(Enum) _character (Variables|Default|GetCharacter))
    (Components|SkinnedMesh|SetSkinnedAssetandUpdate (Variables|Character|GetMesh) _headmesh true)
    (Components|SkinnedMesh|SetSkinnedAssetandUpdate (Variables|Default|GetBody_Chest) _chestmesh true)
    (Components|SkinnedMesh|SetSkinnedAssetandUpdate (Variables|Default|GetBody_Arms) _armsmesh true)
    (Components|SkinnedMesh|SetSkinnedAssetandUpdate (Variables|Default|GetBody_Hands) _handsmesh true)
    (Components|SkinnedMesh|SetSkinnedAssetandUpdate (Variables|Default|GetBody_Legs) _legsmesh true)
    (Components|SkinnedMesh|SetSkinnedAssetandUpdate (Variables|Default|GetBody_Feet) _feetmesh true)
    (Class|SkeletalMeshComponent|SetAnimClass (Variables|Character|GetMesh) _animbp)))

(fn SetVisibilitytoSlot
  (params (SlotName :type Name) (Visibility :type Boolean))
  (if (CallFunction|IsUseMaterialSlots)
    (switch name SlotName
      (:BODY_CHEST
        (LocalVariables|Set_FindString "chest"))
      (:BODY_ARMS
        (LocalVariables|Set_FindString "arms"))
      (:BODY_HANDS
        (LocalVariables|Set_FindString "hands"))
      (:BODY_LEGS
        (LocalVariables|Set_FindString "legs"))
      (:BODY_FEET
        (LocalVariables|Set_FindString "feet"))
      (:BODY_MESH
        (LocalVariables|Set_FindString "head")))
    (for (_array_element _array_index) (Variables|/Script/Engine.SkeletalMesh|GetMaterials (Variables|/Script/Engine.SkeletalMeshComponent|GetSkeletalMeshAsset (Variables|Character|GetMesh)))
      (if (Utilities|String|Contains (Utilities|String|ToString(Name) (.MaterialSlotName (Utilities|Struct|BreakSkeletalMaterial _array_element))) (LocalVariables|Get_FindString))
        (Class|SkinnedMeshComponent|ShowMaterialSection (Variables|Character|GetMesh) _array_index 0 Visibility)))
    (else
      (for _array_element_2 (Actor|GetComponentsbyTag "/Script/Engine.SkeletalMeshComponent" SlotName)
        (Development|SetHiddeninGame _array_element_2 (not Visibility) false)))))

(fn SetUseMaterialSlots
  (params (UseMaterialSlot :type Boolean))
  (Variables|Default|SetUseMaterialSlot UseMaterialSlot)
  (CallFunction|UpdateMesh))

(fn ClampbyRange
  (params (Value :type Float%20%28double-precision%29) (Range :type Float%20Range%20Structure%20%28by%20ref%29))
  (bind (_lowerbound _upperbound) (Utilities|Struct|BreakFloatRange Range))
  (return (Math|Float|Clamp(Float) Value (Utilities|Struct|BreakFloatRangeBound _lowerbound) (Utilities|Struct|BreakFloatRangeBound _upperbound))))

(fn GetClothComponent
  (return (Variables|Default|GetBPC_ClothComponent)))