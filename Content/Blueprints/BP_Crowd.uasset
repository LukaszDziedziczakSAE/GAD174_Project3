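; BP_Crowd is a modular skeletal-mesh character, apparently a crowd member, that varies its outfit at spawn.
; On BeginPlay it picks a random integer and switches the Robe component to one of eight light chest mesh variants in different styles and colors.
; The construction script makes the head and hands meshes follow the Robe as leader pose component, so one skeleton drives all parts.
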(event EventBeginPlay
  (bind _robe (Variables|Default|GetRobe))
  (switch int (Math|Random|RandomIntegerinRange 0 7)
    (:0
      (Components|SkeletalMesh|SetSkeletalMeshAsset _robe "/Game/ROG_Modular_Armor/Accessories_Robes/UE5_Mannequins/Manny/Robes/SkeletalMeshes/SK_Chest2_Light_T1_white.SK_Chest2_Light_T1_white"))
    (:1
      (Components|SkeletalMesh|SetSkeletalMeshAsset _robe "/Game/ROG_Modular_Armor/Accessories_Robes/UE5_Mannequins/Manny/Robes/SkeletalMeshes/SK_Chest2_Light_T1.SK_Chest2_Light_T1"))
    (:2
      (Components|SkeletalMesh|SetSkeletalMeshAsset _robe "/Game/ROG_Modular_Armor/Accessories_Robes/UE5_Mannequins/Manny/Robes/SkeletalMeshes/SK_Chest2_Light_T2.SK_Chest2_Light_T2"))
    (:3
      (Components|SkeletalMesh|SetSkeletalMeshAsset _robe "/Game/ROG_Modular_Armor/Accessories_Robes/UE5_Mannequins/Manny/Robes/SkeletalMeshes/SK_Chest2_Light_T1_green.SK_Chest2_Light_T1_green"))
    (:4
      (Components|SkeletalMesh|SetSkeletalMeshAsset _robe "/Game/ROG_Modular_Armor/Accessories_Robes/UE5_Mannequins/Manny/Robes/SkeletalMeshes/SK_Chest2_Light_T1_red.SK_Chest2_Light_T1_red"))
    (:5
      (Components|SkeletalMesh|SetSkeletalMeshAsset _robe "/Game/ROG_Modular_Armor/Accessories_Robes/UE5_Mannequins/Manny/Robes/SkeletalMeshes/SK_Chest2_Light_T2_green.SK_Chest2_Light_T2_green"))
    (:6
      (Components|SkeletalMesh|SetSkeletalMeshAsset _robe "/Game/ROG_Modular_Armor/Accessories_Robes/UE5_Mannequins/Manny/Robes/SkeletalMeshes/SK_Chest2_Light_T2_red.SK_Chest2_Light_T2_red"))
    (:7
      (Components|SkeletalMesh|SetSkeletalMeshAsset _robe "/Game/ROG_Modular_Armor/Accessories_Robes/UE5_Mannequins/Manny/Robes/SkeletalMeshes/SK_Chest2_Light_T2_white.SK_Chest2_Light_T2_white"))))

(event Collision|EventActorBeginOverlap
  (params (OtherActor :type Actor%20Object%20Reference)))

(event EventTick
  (params (DeltaSeconds :type Float%20%28single-precision%29)))

(fn ConstructionScript
  (Components|SkinnedMesh|SetLeaderPoseComponent (Variables|Default|GetSK_Military_Head1) (Variables|Default|GetRobe) false false))